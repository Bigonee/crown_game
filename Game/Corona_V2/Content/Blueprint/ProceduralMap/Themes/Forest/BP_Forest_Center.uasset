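; BP_Forest_Center is the center piece of the Forest theme for the procedural map.
; Its construction script moves AttachPoint to the AttachPointLocation variable, and GetAttachPointTransform simply returns the parent implementation's result.
; On BeginPlay, SpawnAssets calls SpawnCar, which spawns one EnemyPawn_cars at the SPLeftCar component's world transform with this actor as owner.
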(event EventBeginPlay
  (CallFunction|SpawnAssets))

(event Collision|EventActorBeginOverlap
  (params (OtherActor :type Actor%20Object%20Reference)))

(event EventTick
  (params (DeltaSeconds :type Float%20%28single-precision%29)))

(fn ConstructionScript
  (Transformation|SetRelativeLocation (Variables|Default|GetattachPoint) (Variables|Default|GetattachPointLocation) false false))

(fn GetAttachPointTransform
  (bind _attachtransform (|CallParentFunction))
  (return _attachtransform))

(fn SpawnAssets
  (CallFunction|SpawnCar))

(fn SpawnCar
  (Game|SpawnActorfromClass "/Game/Blueprint/Enemies/Vehicles/EnemyPawn_cars.EnemyPawn_cars_C" (Transformation|GetWorldTransform (Variables|Default|GetSP_Left_Car)) "Undefined" self "NewEnumerator0" 0))