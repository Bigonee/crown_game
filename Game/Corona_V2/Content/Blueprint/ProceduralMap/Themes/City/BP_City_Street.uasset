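; City street segment for the procedural map's City theme, which populates itself with enemies and houses on BeginPlay.
; The construction script positions the attach point, while the attach transform getter defers to the parent class.
; Car, citizen and group enemy pawns each spawn at their own spawn point.
; Houses are static mesh components added at six house points, with a leftover debug print for each.
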(event EventBeginPlay
  (CallFunction|SetSpawnPoints)
  (CallFunction|SpawnAssets))

(event Collision|EventActorBeginOverlap
  (params (OtherActor :type Actor%20Object%20Reference)))

(event EventTick
  (params (DeltaSeconds :type Float%20%28single-precision%29)))

(fn ConstructionScript
  (Transformation|SetRelativeLocation (Variables|Default|GetattachPoint) (Variables|Default|GetattachPointLocation) false false))

(fn GetAttachPointTransform
  (bind _attachtransform (|CallParentFunction))
  (return _attachtransform))

(fn SpawnAssets
  (Utilities|FlowControl|Sequence
    (:then_0
      (CallFunction|SpawnCar))
    (:then_1
      (CallFunction|SpawnCitzen))
    (:then_2
      (CallFunction|SpawnGroup))
    (:then_3
      (CallFunction|SpawnHouses))))

(fn SpawnCar
  (Game|SpawnActorfromClass "/Game/Blueprint/Enemies/Vehicles/EnemyPawn_cars.EnemyPawn_cars_C" (Transformation|GetWorldTransform (Variables|Default|GetSP_Car)) "Undefined" self "NewEnumerator0" 0))

(fn SpawnCitzen
  (Game|SpawnActorfromClass "/Game/Blueprint/Enemies/Citizens/EnemyPawn_Citizen.EnemyPawn_Citizen_C" (Transformation|GetWorldTransform (Variables|Default|GetSP_Citzen)) "Undefined" self "NewEnumerator5" 0))

(fn SpawnGroup
  (Game|SpawnActorfromClass "/Game/Blueprint/Enemies/Groups/EnemyPawn_Group.EnemyPawn_Group_C" (Transformation|GetWorldTransform (Variables|Default|GetSP_Group)) "Undefined" self "NewEnumerator4" 0))

(fn SpawnHouses
  (for _array_element (Variables|Default|GetspHouses2)
    (Development|PrintString "Hello")
    (AddComponent|AddStaticMeshComponent false (Transformation|GetRelativeTransform _array_element))))

(fn SetSpawnPoints
  (Utilities|FlowControl|Sequence
    (:then_0
      (CallFunction|SetSpawnPointsforHouses))))

(fn SetSpawnPointsforHouses
  (Variables|Default|SetspHouses2 (Utilities|Array|MakeArray (Variables|Default|GetSP_House_1) (Variables|Default|GetSP_House_2) (Variables|Default|GetSP_House_3) (Variables|Default|GetSP_House_4) (Variables|Default|GetSP_House_8) (Variables|Default|GetSP_House_7))))