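; Street tile for the procedural map, with a street mesh, two sidewalks and an attach point, dressed in a city or desert theme.
; The construction script positions the attach point and swaps the three meshes to match the Theme.
; GetAttachPointTransform simply defers to the parent class.
; On BeginPlay the tile spawns an enemy car pawn at its left car spawn point, with itself as owner.
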(event EventBeginPlay
  (CallFunction|SpawnAssets))

(event Collision|EventActorBeginOverlap
  (params (OtherActor :type Actor%20Object%20Reference)))

(event EventTick
  (params (DeltaSeconds :type Float%20%28single-precision%29)))

(fn ConstructionScript
  (Utilities|FlowControl|Sequence
    (:then_0
      (Transformation|SetRelativeLocation (Variables|Default|GetattachPoint) (Variables|Default|GetattachPointLocation) false false))
    (:then_1
      (switch Utilities|FlowControl|Switch|SwitchonEN_TileTheme (Variables|Default|Gettheme)
        (:NewEnumerator0
          (CallFunction|SetCityTheme))
        (:NewEnumerator1
          (CallFunction|SetDesertTheme))))))

(fn GetAttachPointTransform
  (bind _attachtransform (|CallParentFunction))
  (return _attachtransform))

(fn SetCityTheme
  (Utilities|FlowControl|Sequence
    (:then_0
      (Components|StaticMesh|SetStaticMesh (Variables|Default|GetStreetMesh) "/Game/ImportedMesh/CITY/center_city.center_city"))
    (:then_1
      (Components|StaticMesh|SetStaticMesh (Variables|Default|GetSidewalkLeft) "/Game/ImportedMesh/CITY/sidewalk_left_city.sidewalk_left_city"))
    (:then_2
      (Components|StaticMesh|SetStaticMesh (Variables|Default|GetSidewalkRight) "/Game/ImportedMesh/CITY/sidewalk_right_city.sidewalk_right_city"))))

(fn SetDesertTheme
  (Utilities|FlowControl|Sequence
    (:then_0
      (Components|StaticMesh|SetStaticMesh (Variables|Default|GetStreetMesh) "/Game/ImportedMesh/DESERT/center_desert.center_desert"))
    (:then_1
      (Components|StaticMesh|SetStaticMesh (Variables|Default|GetSidewalkLeft) "/Game/ImportedMesh/DESERT/sidewalk_left_desert.sidewalk_left_desert"))
    (:then_2
      (Components|StaticMesh|SetStaticMesh (Variables|Default|GetSidewalkRight) "/Game/ImportedMesh/DESERT/sidewalk_right_desert.sidewalk_right_desert"))))

(fn SpawnAssets
  (CallFunction|SpawnCar))

(fn SpawnCar
  (Game|SpawnActorfromClass "/Game/Blueprint/Enemies/Vehicles/EnemyPawn_cars.EnemyPawn_cars_C" (Transformation|GetWorldTransform (Variables|Default|GetSP_Left_Car)) "Undefined" self "NewEnumerator0" 0))