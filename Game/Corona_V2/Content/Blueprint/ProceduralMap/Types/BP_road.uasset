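; BP_road is a road tile Blueprint for procedural map generation.
; Its construction script positions the attach point, sets the street mesh and stores two confined points in an array.
; It also sorts "SP"-tagged arrow components by secondary tag into vehicle, citizen, trash and group spawn arrays.
; The tile-number parity check has empty branches, so every tile gets the same Road_type_2 mesh.
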(event Collision|EventActorBeginOverlap
  (params (OtherActor :type Actor%20Object%20Reference))
  (|CallParentFunction OtherActor) ; This node is disabled and will not be called.\nDrag off pins to build functionality.
)

(event EventTick
  (params (DeltaSeconds :type Float%20%28single-precision%29))
  (|CallParentFunction DeltaSeconds) ; This node is disabled and will not be called.\nDrag off pins to build functionality.
)

(event EventSetConfinedPoints
  (Variables|Default|SetcpConfined (Utilities|Array|MakeArray (Variables|Default|Getconfined_point_1) (Variables|Default|Getconfined_point_2))))

(event EventBeginPlay
  (|CallParentFunction))

(event EventSetSpawnPoints)

(fn ConstructionScript
  (|CallParentFunction)
  (Utilities|FlowControl|Sequence
    (:then_0
      (CallFunction|SetupTileTypeMesh))
    (:then_1
      (CallFunction|SetupSpawnPointsArray))
    (:then_2
      (Variables|Default|SetcpConfined (Utilities|Array|MakeArray (Variables|Default|Getconfined_point_1) (Variables|Default|Getconfined_point_2))))))

(fn SetupTileTypeMesh
  (Transformation|SetRelativeLocation (Variables|Default|GetattachPoint) (Variables|Default|GetattachPointVar) false false)
  (if (== (Math|Float|Truncate (.Remainder (Math|Float|Division(WholeandRemainder) (Math|Conversions|ToFloat(Integer) (Variables|Default|GettileNumber)) 2.0))) 0)
    _
    (else
      _))
  (Components|StaticMesh|SetStaticMesh (Variables|Default|Getstreet_mesh) "/Game/TileMesh/Road/road_type_2.road_type_2"))

(fn SetupSpawnPointsArray
  (for _array_element (Actor|GetComponentsbyTag "/Script/Engine.ActorComponent" "SP")
    (bind _asarrow_component (Utilities|Casting|CastToArrowComponent _array_element))
    (Utilities|FlowControl|Sequence
      (:then_0
        (if (Components|ComponentHasTag _array_element "SP_VEHICLE")
          (Utilities|Array|Add (Variables|Default|GetspCarsArray) _asarrow_component)))
      (:then_1
        (if (Components|ComponentHasTag _array_element "SP_CITZEN")
          (Utilities|Array|Add (Variables|Default|GetspCharactersArray) _asarrow_component)))
      (:then_2
        (if (Components|ComponentHasTag _array_element "SP_TRASH")
          (Utilities|Array|Add (Variables|Default|GetspTrashArray) _asarrow_component)))
      (:then_3
        (if (Components|ComponentHasTag _array_element "SP_GROUP")
          (Utilities|Array|Add (Variables|Default|GetspGroupsArray) _asarrow_component))))))