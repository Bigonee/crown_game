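; BP_crossroad is a crossroad piece type for the procedural map.
; Its construction script moves the AttachPoint component to the AttachPointVar location and assigns the Crossroad_1 mesh to the CrossroadType3 component.
; SpawnAssets is an empty function, and the event graph holds only disabled default events, so the piece has no runtime logic of its own.
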(event EventBeginPlay
  (|CallParentFunction) ; This node is disabled and will not be called.\nDrag off pins to build functionality.
)

(event Collision|EventActorBeginOverlap
  (params (OtherActor :type Actor%20Object%20Reference))
  (|CallParentFunction OtherActor) ; This node is disabled and will not be called.\nDrag off pins to build functionality.
)

(event EventTick
  (params (DeltaSeconds :type Float%20%28single-precision%29))
  (|CallParentFunction DeltaSeconds) ; This node is disabled and will not be called.\nDrag off pins to build functionality.
)

(fn ConstructionScript
  (Transformation|SetRelativeLocation (Variables|Default|GetattachPoint) (Variables|Default|GetattachPointVar) false false)
  (Components|StaticMesh|SetStaticMesh (Variables|Default|Getcrossroad_type_3) "/Game/TileMesh/CrossRoad/crossroad_1.crossroad_1"))

(fn SpawnAssets)