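; EnemyPawn is an enemy pawn Blueprint that exposes tap state, damage and infection values through simple functions.
; CallEnemyTap flags the enemy as tapped and returns its ExtraPoints, while AskHasBeenTap reports that flag.
; GetDamageAmount and GetInfectionAmount are plain getters for Damage and Infection.
; MakeDamage is empty, ElementClean always returns zero, and the event graph and construction script hold no active logic.
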(event EventBeginPlay)

(event Collision|EventActorBeginOverlap
  (params (OtherActor :type Actor%20Object%20Reference)))

(event EventTick
  (params (DeltaSeconds :type Float%20%28single-precision%29)))

(fn ConstructionScript)

(fn MakeDamage)

(fn AskHasBeenTap
  (return (Variables|Default|GethasBeenTap)))

(fn CallEnemyTap
  (Variables|Default|SethasBeenTap true)
  (return (Variables|Default|GetextraPoints)))

(fn ElementClean
  (return 0))

(fn GetDamageAmount
  (return (Variables|Default|Getdamage)))

(fn GetInfectionAmount
  (return (Variables|Default|Getinfection)))