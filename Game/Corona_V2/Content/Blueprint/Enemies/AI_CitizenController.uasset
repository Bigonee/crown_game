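; AI controller for a citizen pawn that keeps it walking straight ahead until it is sent to a specific point.
; On BeginPlay a fast looping timer repeatedly moves the pawn to a spot just ahead along its forward vector, without pathfinding.
; The goToConfinedPoint event clears that timer and moves the pawn directly to the given destination, also without pathfinding.
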(event Custom|goToConfinedPoint
  (params (Dest :type Vector%20%28by%20ref%29))
  (Utilities|Time|ClearandInvalidateTimerbyHandle (Variables|Default|GetwalkForwardTimer))
  (AI|Navigation|MovetoLocation Dest 0.0 false false false true 0))

(event Custom|WalkForward
  (bind _returnvalue (Pawn|GetControlledPawn))
  (AI|Navigation|MovetoLocation (+ (Transformation|GetActorLocation _returnvalue) (* (Transformation|GetActorForwardVector _returnvalue) 8e+01)) 0.0 true false false true 0))

(event EventBeginPlay
  (bind _returnvalue (Utilities|Time|SetTimerbyEvent (delegate Custom|WalkForward) 0.1 true))
  (Variables|Default|SetwalkForwardTimer _returnvalue))

(event EventTick
  (params (DeltaSeconds :type Float%20%28single-precision%29)))

(fn ConstructionScript)