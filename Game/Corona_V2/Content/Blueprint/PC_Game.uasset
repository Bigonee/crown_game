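; Player controller for an endless-runner level, handling HUD, input, scoring and game over.
; The horizontal widget's buttons and action mappings forward movement and abilities to the pawn via messages.
; A looping timer sums pawn distance and extra points, which grow from trash cleanup and combo-multiplied enemy taps but reset when combos end.
; Zero HP, maximum infection or beach death saves the score, shows results and submits to leaderboards.
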(event Custom|EndCombo
  ;[1 1 1] Touch Sreen to interact Enemies
  (Points|FinishCombo)
  (Utilities|Time|ClearandInvalidateTimerbyHandle (Variables|PointSystem|GetComboTimer)))

(event Custom|UpdateUIHabilities
  (bind _returnvalue (Game|Player|GetPlayerPawn 0))
  (bind _ingameui_horizontal (Variables|Default|GetInGameUI_Horizontal))
  ;[1 1 1] Begin Play Logic
  (Utilities|FlowControl|Sequence
    (:then_0
      ;[1 1 1] Hability - UPDATE UI DATA
      (bind (_en_habilitydurationstate _charge) (Class|PawnInterface|RequestHabilityDurationData(Message) _returnvalue))
      (Default|UpdateHabilityDurationUIData _ingameui_horizontal _en_habilitydurationstate _charge 0.0))
    (:then_1
      (bind _bullets (Class|PawnInterface|RequestHability1useData(Message) _returnvalue))
      (Default|UpdateBullets _ingameui_horizontal _bullets))))

(event Custom|Replay
  ;[1 1 1] POPUP UI Buttons
  (Game|OpenLevel(byName) "EndlessMap_Mobile"))

(event Custom|GoToMenu
  ;[1 1 1] POPUP UI Buttons
  (Game|OpenLevel(byName) "MainMap"))

(event Custom|Leaderboard
  ;[1 1 1] POPUP UI Buttons
)

(event Custom|UpdatePointsUI
  (bind _distancepoints (Variables|PointSystem|GetDistancePoints))
  (bind _extrapoints (Variables|PointSystem|GetExtraPoints))
  (bind _returnvalue (+ _distancepoints _extrapoints))
  ;[1 1 1] Begin Play Logic
  (Points|IncrementPointsinDistance)
  (Variables|PointSystem|SetTotalScore _returnvalue)
  (Default|UpdateCurrentPoints (Variables|Default|GetInGameUI_Horizontal) _returnvalue))

(event EventBeginPlay
  ;[1 1 1] Begin Play Logic
  (Variables|Default|SetbShowMouseCursor true)
  (Utilities|FlowControl|Sequence
    (:then_0
      (CallFunction|CreateSaveLoadController))
    (:then_1
      (|WIDGETStuff-Horizontal))
    (:then_2
      (Default|UpdatePointsHPProgressBars (Variables|Default|GetInGameUI_Horizontal) 100))
    (:then_3
      (bind _returnvalue (Utilities|Time|SetTimerbyEvent (delegate Custom|UpdatePointsUI) 0.1 true))
      (Variables|PointSystem|SetPointTrackerEventTimer _returnvalue))
    (:then_4
      (Audio|PlaySound2D "/Game/Sounds/src/background/bensound-jazzyfrenchy_Cue.bensound-jazzyfrenchy_Cue" 0.25 1.0 0.0 0 self))))

(event EventCallWarningMessage
  (params (WarningMessage :type Text))
  ;[1 1 1] Warning Messages
  (Default|SetupandShowWarningMessage (Variables|Default|GetInGameUI_Horizontal) WarningMessage))

(event EventUpdateHpInfection
  (params (HP :type Integer) (Infection :type Integer))
  (bind _ingameui_horizontal (Variables|Default|GetInGameUI_Horizontal))
  ;[1 1 1] HP - Infection Data Flow
  (Utilities|IsValid _ingameui_horizontal
    (:Is%20Valid
      (Default|UpdatePointsHPProgressBars _ingameui_horizontal HP Infection)
      (bind _returnvalue (CallFunction|CheckifEndGame HP Infection))
      ;[1 1 1] On Die Execution
      (if _returnvalue
        ;;[1 0.832 0.4972] Send Data To server (Local Now)
        (Default|SavePointsData (Variables|Default|GetSaveGameController) (Math|Conversions|ToFloat(Integer) (Variables|PointSystem|GetTotalScore)))
        ;;[1 1 1] Disable Movement INPUT
        (Class|PawnInterface|OnDieEndGame(Message) (Game|Player|GetPlayerPawn 0))
        (Default|SetupEndGame (Variables|Default|GetInGameUI_Horizontal) (Variables|PointSystem|GetTotalTapConfined) (Variables|PointSystem|GetTotalTrashClean) (Math|Conversions|ToFloat(Integer) (Variables|PointSystem|GetDistancePoints)) (Math|Conversions|ToFloat(Integer) (Variables|PointSystem|GetTotalScore)))
        (Utilities|Time|ClearandInvalidateTimerbyHandle (Variables|PointSystem|GetPointTrackerEventTimer))
        (Utilities|FlowControl|DoOnce false
          (:Completed
            (Points|SendDatatoServer)))))))

(event EventPickUpBooster
  ;[1 1 1] UI Boosta
  (Default|SetupandShowWarningMessage (Variables|Default|GetInGameUI_Horizontal) "GAS BOOOOSTAH!!!"))

(event EventAddCleanedVirusCounter
  (params (EnemyPoints :type Integer))
  ;[1 1 1] Add Cleaned Trash
  (Variables|PointSystem|SetTotalTrashClean (+ (Variables|PointSystem|GetTotalTrashClean) 1))
  (Variables|PointSystem|SetExtraPoints (+ (Variables|PointSystem|GetExtraPoints) EnemyPoints)))

(event EventDieonBeach
  ;[1 1 1] Die On Beach
  ;[1 1 1] On Die Execution
  ;;[1 0.832 0.4972] Send Data To server (Local Now)
  (Default|SavePointsData (Variables|Default|GetSaveGameController) (Math|Conversions|ToFloat(Integer) (Variables|PointSystem|GetTotalScore)))
  ;;[1 1 1] Disable Movement INPUT
  (Class|PawnInterface|OnDieEndGame(Message) (Game|Player|GetPlayerPawn 0))
  (Default|SetupEndGame (Variables|Default|GetInGameUI_Horizontal) (Variables|PointSystem|GetTotalTapConfined) (Variables|PointSystem|GetTotalTrashClean) (Math|Conversions|ToFloat(Integer) (Variables|PointSystem|GetDistancePoints)) (Math|Conversions|ToFloat(Integer) (Variables|PointSystem|GetTotalScore)))
  (Utilities|Time|ClearandInvalidateTimerbyHandle (Variables|PointSystem|GetPointTrackerEventTimer))
  (Utilities|FlowControl|DoOnce false
    (:Completed
      (Points|SendDatatoServer))))

(event Input|TouchEvents|Touch2
  (params (Key :type Key%20Structure))
  (bind _hitresult (Game|Player|GetHitResultUnderCursorbyChannel "TraceTypeQuery1" true))
  (bind (_bblockinghit _binitialoverlap _time _distance _location _impactpoint _normal _impactnormal _physmat _hitactor) (Collision|BreakHitResult _hitresult))
  ;[1 1 1] Touch Sreen to interact Enemies
  (:Pressed
    (if _bblockinghit
      (if (Actor|ActorHasTag _hitactor "tappable")
        (bind _hasbeentap (Class|EnemyInterface|AskHasBeenTap(Message) _hitactor))
        (if (not _hasbeentap)
          ;;[1 0.8512 0.4328] Output enemy type in order to count totals in score pop up screen
          (bind _extrapoints (Class|EnemyInterface|CallEnemyTap(Message) _hitactor))
          (Points|ProcessExtraPoints _extrapoints)
          (Points|DrawExtraPointsPopUp)
          (Points|IncrementComboTimeonTap)
          (bind _returnvalue (Utilities|Time|SetTimerbyEvent (delegate Custom|EndCombo) (Variables|PointSystem|GetComboTimeLimit)))
          (Variables|PointSystem|SetComboTimer _returnvalue))))))

(event Input|TouchEvents|Touch1
  (params (Key :type Key%20Structure))
  (bind _hitresult (Game|Player|GetHitResultUnderCursorbyChannel "TraceTypeQuery1" true))
  (bind (_bblockinghit _binitialoverlap _time _distance _location _impactpoint _normal _impactnormal _physmat _hitactor) (Collision|BreakHitResult _hitresult))
  ;[1 1 1] Touch Sreen to interact Enemies
  (:Pressed
    (if _bblockinghit
      (if (Actor|ActorHasTag _hitactor "tappable")
        (bind _hasbeentap (Class|EnemyInterface|AskHasBeenTap(Message) _hitactor))
        (if (not _hasbeentap)
          ;;[1 0.8512 0.4328] Output enemy type in order to count totals in score pop up screen
          (bind _extrapoints (Class|EnemyInterface|CallEnemyTap(Message) _hitactor))
          (Points|ProcessExtraPoints _extrapoints)
          (Points|DrawExtraPointsPopUp)
          (Points|IncrementComboTimeonTap)
          (bind _returnvalue (Utilities|Time|SetTimerbyEvent (delegate Custom|EndCombo) (Variables|PointSystem|GetComboTimeLimit)))
          (Variables|PointSystem|SetComboTimer _returnvalue))))))

(fn ConstructionScript)

(fn CheckifEndGame
  (params (HP :type Integer) (InfectionAmount :type Integer))
  (return (or (<= HP 0) (>= InfectionAmount (Variables|Default|GetMaxInfectionValue)))))

(fn CreateSaveLoadController
  (Utilities|IsValid (Variables|Default|GetSaveGameController)
    (:Is%20Not%20Valid
      (bind _returnvalue (Game|ConstructObjectfromClass "/Game/Blueprint/SaveGame/SaveGameController.SaveGameController_C" self))
      (Variables|Default|SetSaveGameController _returnvalue))))

(fn IncrementPointsinDistance
  (bind _distanceamount (Class|PawnInterface|GetDistance(Message) (Pawn|GetControlledPawn)))
  (Variables|PointSystem|SetDistancePoints (Math|Float|Truncate _distanceamount)))

(fn ProcessExtraPoints
  (params (ExtraPoint :type Integer))
  (Variables|PointSystem|SetTotalTapConfined (+ (Variables|PointSystem|GetTotalTapConfined) 1))
  (Variables|PointSystem|SetComboTapNumber (+ (Variables|PointSystem|GetComboTapNumber) 1))
  (Variables|PointSystem|SetExtraPoints (+ (* ExtraPoint (Variables|PointSystem|GetComboTapNumber)) (Variables|PointSystem|GetExtraPoints))))

(fn DrawExtraPointsPopUp
  (Default|UpdateExtraPointsWdg (Variables|Default|GetInGameUI_Horizontal) (Variables|PointSystem|GetExtraPoints) (Variables|PointSystem|GetComboTapNumber)))

(fn FinishCombo
  (Variables|PointSystem|SetExtraPoints 0)
  (Variables|PointSystem|SetComboTapNumber 0)
  (Default|FinishCombo (Variables|Default|GetInGameUI_Horizontal)))

(fn IncrementComboTimeonTap
  (if (>= (+ (Variables|PointSystem|GetComboTimeLimit) (Variables|PointSystem|GetComboTimeIncrementOnTap)) (Variables|PointSystem|GetComboTimeIncrementOnTap))
    (Variables|PointSystem|SetComboTimeLimit 2.0)
    (else
      (Variables|PointSystem|SetComboTimeLimit (+ (Variables|PointSystem|GetComboTimeLimit) (Variables|PointSystem|GetComboTimeIncrementOnTap))))))

(fn SendDatatoServer
  (bind _totalscore (Variables|PointSystem|GetTotalScore))
  (bind _asgame_instance_corona (Utilities|Casting|CastToGameInstanceCorona (Game|GetGameInstance)))
  (Default|SubmitScore (Variables|Default|GetInGameUI_Horizontal) (Variables|/Game/Blueprint/GameInstanceCorona.GameInstanceCorona_C|GetUserName _asgame_instance_corona) (Math|Conversions|ToFloat(Integer) _totalscore))
  (bind _returnvalue (Class|LeaderboardBlueprintLibrary|WriteLeaderboardInteger (Game|GetPlayerController 0) "Project_C_Score" _totalscore)))

(fn CallCleanAction
  (Class|PawnInterface|CallHabilityDuration(Message) (Pawn|GetControlledPawn)))

(fn CallHealAction
  (Class|PawnInterface|CallHabilityShoot(Message) (Pawn|GetControlledPawn)))

(fn SetupWdgHabilityCleanState
  (params (EN_HabilityDurationState :type EN_HabilityDurationState%20Enum :default "NewEnumerator0")))

(fn CallHabilityDuration
  (return "NewEnumerator0"))

(event Custom|MoveRight_Event_0
  (params (isPressed :type Boolean))
  ;[1 1 1] Move Actions
  (Class|PawnInterface|CallMoveRight(Message) (Game|Player|GetPlayerPawn 0) isPressed))

(event Custom|MoveLeft_Event_0
  (params (isPressed :type Boolean))
  ;[1 1 1] Move Actions
  (Class|PawnInterface|CallMoveLeft(Message) (Game|Player|GetPlayerPawn 0) isPressed))

(event Custom|Jump_Event_0
  (params (isPressed :type Boolean))
  ;[1 1 1] Move Actions
  (Class|PawnInterface|CallJump(Message) (Game|Player|GetPlayerPawn 0) isPressed))

(event Custom|GoToMenu_Event_0
  ;[1 1 1] On Die PopUp UI
  (CallFunction|GotoMenu))

(event Custom|Replay_Event_0
  ;[1 1 1] On Die PopUp UI
  (CallFunction|Replay))

(event Custom|Leaderboard_Event_0
  ;[1 1 1] On Die PopUp UI
  (CallFunction|Leaderboard))

(event Custom|PerkLeft_Event_0
  ;[1 1 1] Perks Actions
  (HabilityActiveDuration|CallHealAction))

(event Custom|PerkRight_Event_0
  ;[1 1 1] Perks Actions
  (HabilityActiveDuration|CallCleanAction))

(event Input|ActionEvents|InputActionMoveLeft
  (params (Key :type Key%20Structure))
  ;[1 1 1] INPUT WITH BUTTONS (PC - CONSOLE)
)

(event Input|ActionEvents|InputActionMoveRight
  (params (Key :type Key%20Structure))
  ;[1 1 1] INPUT WITH BUTTONS (PC - CONSOLE)
)

(event Input|ActionEvents|InputActionJump
  (params (Key :type Key%20Structure))
  ;[1 1 1] INPUT WITH BUTTONS (PC - CONSOLE)
)

(event Input|ActionEvents|InputActionActiveClean
  (params (Key :type Key%20Structure))
  ;[1 1 1] INPUT WITH BUTTONS (PC - CONSOLE)
)

(event Input|ActionEvents|InputActionActiveShoot
  (params (Key :type Key%20Structure))
  ;[1 1 1] INPUT WITH BUTTONS (PC - CONSOLE)
)

(event Custom|CustomEvent
  (params (isPressed :type Boolean))
  ;[1 1 1] Move Actions
  (Class|PawnInterface|CallMoveRight(Message) (Game|Player|GetPlayerPawn 0) isPressed))

(event Custom|CustomEvent_1
  (params (isPressed :type Boolean))
  ;[1 1 1] Move Actions
  (Class|PawnInterface|CallMoveLeft(Message) (Game|Player|GetPlayerPawn 0) isPressed))

(event Custom|CustomEvent_2
  (params (isPressed :type Boolean))
  ;[1 1 1] Move Actions
  (Class|PawnInterface|CallJump(Message) (Game|Player|GetPlayerPawn 0) isPressed))

(event Custom|CustomEvent_3
  ;[1 1 1] On Die PopUp UI
  (CallFunction|GotoMenu))

(event Custom|CustomEvent_4
  ;[1 1 1] On Die PopUp UI
  (CallFunction|Replay))

(event Custom|CustomEvent_5
  ;[1 1 1] On Die PopUp UI
  (CallFunction|Leaderboard))

(event Custom|CustomEvent_6
  ;[1 1 1] Perks Actions
  (HabilityActiveDuration|CallHealAction))

(event Custom|CustomEvent_7
  ;[1 1 1] Perks Actions
  (HabilityActiveDuration|CallCleanAction))

(event Input|ActionEvents|InputActionJump
  (params (Key :type Key%20Structure))
  (bind _returnvalue (Game|Player|GetPlayerPawn 0))
  ;[1 1 1] INPUT WITH BUTTONS (PC - CONSOLE)
  (:Pressed
    (Class|PawnInterface|CallJump(Message) _returnvalue true))
  (:Released
    (Class|PawnInterface|CallJump(Message) _returnvalue false)))

(event Input|ActionEvents|InputActionActiveClean
  (params (Key :type Key%20Structure))
  ;[1 1 1] INPUT WITH BUTTONS (PC - CONSOLE)
)

(event Input|ActionEvents|InputActionActiveShoot
  (params (Key :type Key%20Structure))
  ;[1 1 1] INPUT WITH BUTTONS (PC - CONSOLE)
)

(event Input|ActionEvents|InputActionMoveUp
  (params (Key :type Key%20Structure))
  (bind _returnvalue (Game|Player|GetPlayerPawn 0))
  ;[1 1 1] INPUT WITH BUTTONS (PC - CONSOLE)
  (:Pressed
    (Class|PawnInterface|CallMoveLeft(Message) _returnvalue true))
  (:Released
    (Class|PawnInterface|CallMoveLeft(Message) _returnvalue false)))

(event Input|ActionEvents|InputActionMoveDown
  (params (Key :type Key%20Structure))
  (bind _returnvalue (Game|Player|GetPlayerPawn 0))
  ;[1 1 1] INPUT WITH BUTTONS (PC - CONSOLE)
  (:Pressed
    (Class|PawnInterface|CallMoveRight(Message) _returnvalue true))
  (:Released
    (Class|PawnInterface|CallMoveRight(Message) _returnvalue false)))

(fn GetDistance
  (return 0.0))

(fn RequestHability1useData
  (return 0))

(fn RequestHabilityDurationData
  (return "NewEnumerator0" 0.0))