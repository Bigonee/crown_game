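; BP_ActorSpawner continually spawns citizen, vehicle and trash enemy pawns, plus pickups, at random tagged arrow points.
; The construction script sorts arrows into per-category arrays for Main and Special 1 tiles; spawns use the deferred tile type's array.
; A one-second timer shortens enemy intervals down to floors, and each enemy spawn function re-arms its timer to apply them.
; Pickups use a separate fixed timer and height; the Special 1 pickup spawn has no class set.
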(event Custom|ChangeToCross)

(event EventBeginPlay
  (Utilities|Time|SetTimerbyFunctionName 0 "UpdateDifficulty" 1.0 true)
  (CallFunction|SpawnCitizens)
  (CallFunction|SpawnVehicles)
  (CallFunction|SpawnTrash)
  (Utilities|Time|SetTimerbyFunctionName 0 "SpawnPickUp" (Variables|Default|GetspwanTimePickUp) true))

(event Collision|EventActorBeginOverlap
  (params (OtherActor :type Actor%20Object%20Reference)))

(fn ConstructionScript
  (for _array_element (Actor|GetComponentsbyTag "/Script/Engine.ActorComponent" "SP")
    (bind _asarrow_component (Utilities|Casting|CastToArrowComponent _array_element))
    (Utilities|FlowControl|Sequence
      (:then_0
        (Utilities|FlowControl|Sequence
          (:then_0
            (if (Components|ComponentHasTag _array_element "M_SP_VEHICLE")
              (Utilities|Array|Add (Variables|Default|GetspMCarsArray) _asarrow_component)))
          (:then_1
            (if (Components|ComponentHasTag _array_element "M_SP_CITZEN")
              (Utilities|Array|Add (Variables|Default|GetspMCharactersArray) _asarrow_component)))
          (:then_2
            (if (Components|ComponentHasTag _array_element "M_SP_TRASH")
              (Utilities|Array|Add (Variables|Default|GetspMTrashArray) _asarrow_component)))
          (:then_3
            (if (Components|ComponentHasTag _array_element "M_SP_PICKUP")
              (Utilities|Array|Add (Variables|Default|GetspMPickUpArray) _asarrow_component)))))
      (:then_1
        (Utilities|FlowControl|Sequence
          (:then_0
            (if (Components|ComponentHasTag _array_element "S1_SP_VEHICLE")
              (Utilities|Array|Add (Variables|Default|GetspS1CarsArray) _asarrow_component)))
          (:then_1
            (if (Components|ComponentHasTag _array_element "S1_SP_CITZEN")
              (Utilities|Array|Add (Variables|Default|GetspS1CharactersArray) _asarrow_component)))
          (:then_2
            (if (Components|ComponentHasTag _array_element "S1_SP_TRASH")
              (Utilities|Array|Add (Variables|Default|GetspS1TrashArray) _asarrow_component)))
          (:then_3
            (if (Components|ComponentHasTag _array_element "S1_SP_PICKUP")
              (Utilities|Array|Add (Variables|Default|GetspS1PickUpArray) _asarrow_component))))))))

(fn GetSpawnLocations
  (params (Array :type Array%20of%20Scene%20Component%20Object%20References))
  (bind _returnvalue (Utilities|Array|Length Array))
  (bind _returnvalue_2 (Math|Random|RandomInteger _returnvalue))
  (bind _output (Utilities|Array|Get(acopy) Array _returnvalue_2))
  (Utilities|IsValid _output
    (:Is%20Valid
      (return (Transformation|GetWorldTransform _output)))))

(fn UpdateDifficulty
  (Utilities|FlowControl|Sequence
    (:then_0
      (if (>= (Variables|Default|GetspwanTimeCitizens) 0.5)
        (Variables|Default|SetspwanTimeCitizens (- (Variables|Default|GetspwanTimeCitizens) 0.01))))
    (:then_1
      (if (>= (Variables|Default|GetspwanTimeVehicles) 2.0)
        (Variables|Default|SetspwanTimeVehicles (- (Variables|Default|GetspwanTimeVehicles) 0.2))))
    (:then_2
      (if (>= (Variables|Default|GetspwanTimeTrash) 1.0)
        (Variables|Default|SetspwanTimeTrash (- (Variables|Default|GetspwanTimeTrash) 0.1))))))

(fn SpawnCitizens
  (Utilities|FlowControl|Sequence
    (:then_0
      (switch Utilities|FlowControl|Switch|SwitchonETileType (Class|MapGen|GetDeferredTileType)
        (:MAIN
          (bind _spawnlocation (CallFunction|GetSpawnLocations (Variables|Default|GetspMCharactersArray)))
          (Game|SpawnActorfromClass "/Game/Blueprint/Enemies/Citizens/EnemyPawn_Citizen.EnemyPawn_Citizen_C" _spawnlocation "Undefined" 0 (Class|MapGen|GetCitzenType (Variables|Default|GettileNumber)) 0))
        (:SPECIAL_1
          (bind _spawnlocation_2 (CallFunction|GetSpawnLocations (Variables|Default|GetspS1CharactersArray)))
          (Game|SpawnActorfromClass "/Game/Blueprint/Enemies/Citizens/EnemyPawn_Citizen.EnemyPawn_Citizen_C" _spawnlocation_2 "Undefined" 0 (Class|MapGen|GetCitzenType (Variables|Default|GettileNumber)) 0))))
    (:then_1
      (if (Utilities|Time|IsValidTimerHandle (Variables|Default|GetSpawnCitizensTimer))
        (Utilities|Time|ClearandInvalidateTimerbyHandle (Variables|Default|GetSpawnCitizensTimer)))
      (bind _returnvalue (Utilities|Time|SetTimerbyFunctionName 0 "SpawnCitizens" (Variables|Default|GetspwanTimeCitizens) true))
      (Variables|Default|SetSpawnCitizensTimer _returnvalue))))

(fn SpawnVehicles
  (Utilities|FlowControl|Sequence
    (:then_0
      (switch Utilities|FlowControl|Switch|SwitchonETileType (Class|MapGen|GetDeferredTileType)
        (:MAIN
          (bind _spawnlocation (CallFunction|GetSpawnLocations (Variables|Default|GetspMCarsArray)))
          (Game|SpawnActorfromClass "/Game/Blueprint/Enemies/Vehicles/EnemyPawn_vehicles.EnemyPawn_Vehicles_C" _spawnlocation "Undefined" 0 (Class|MapGen|GetVehicleType (Variables|Default|GettileNumber)) 0))
        (:SPECIAL_1
          (bind _spawnlocation_2 (CallFunction|GetSpawnLocations (Variables|Default|GetspS1CarsArray)))
          (Game|SpawnActorfromClass "/Game/Blueprint/Enemies/Vehicles/EnemyPawn_vehicles.EnemyPawn_Vehicles_C" _spawnlocation_2 "Undefined" 0 (Class|MapGen|GetVehicleType (Variables|Default|GettileNumber)) 0))))
    (:then_1
      (if (Utilities|Time|IsValidTimerHandle (Variables|Default|GetSpwanVehiclesTimer))
        (Utilities|Time|ClearandInvalidateTimerbyHandle (Variables|Default|GetSpwanVehiclesTimer)))
      (bind _returnvalue (Utilities|Time|SetTimerbyFunctionName 0 "SpawnVehicles" (Variables|Default|GetspwanTimeVehicles) true))
      (Variables|Default|SetSpwanVehiclesTimer _returnvalue))))

(fn SpawnTrash
  (Utilities|FlowControl|Sequence
    (:then_0
      (switch Utilities|FlowControl|Switch|SwitchonETileType (Class|MapGen|GetDeferredTileType)
        (:MAIN
          (bind _spawnlocation (CallFunction|GetSpawnLocations (Variables|Default|GetspMTrashArray)))
          (Game|SpawnActorfromClass "/Game/Blueprint/Enemies/Trash/EnemyPawn_Trash.EnemyPawn_Trash_C" _spawnlocation "Undefined" 0 (Class|MapGen|GetTrashType (Variables|Default|GettileNumber)) 0))
        (:SPECIAL_1
          (bind _spawnlocation_2 (CallFunction|GetSpawnLocations (Variables|Default|GetspS1TrashArray)))
          (Game|SpawnActorfromClass "/Game/Blueprint/Enemies/Trash/EnemyPawn_Trash.EnemyPawn_Trash_C" _spawnlocation_2 "Undefined" 0 (Class|MapGen|GetTrashType (Variables|Default|GettileNumber)) 0))))
    (:then_1
      (if (Utilities|Time|IsValidTimerHandle (Variables|Default|GetSpawnTrashTimer))
        (Utilities|Time|ClearandInvalidateTimerbyHandle (Variables|Default|GetSpawnTrashTimer)))
      (bind _returnvalue (Utilities|Time|SetTimerbyFunctionName 0 "SpawnTrash" (Variables|Default|GetspwanTimeTrash) true))
      (Variables|Default|SetSpawnTrashTimer _returnvalue))))

(fn SpawnPickUp
  (switch Utilities|FlowControl|Switch|SwitchonETileType (Class|MapGen|GetDeferredTileType)
    (:MAIN
      (bind _spawnlocation (CallFunction|GetSpawnLocations (Variables|Default|GetspMPickUpArray)))
      (bind _returnvalue (CallFunction|PickUpOffSet _spawnlocation))
      (bind _returnvalue_2 (Game|SpawnActorfromClass "/Game/Blueprint/PickUp/BP_Pickup_GasBooster.BP_Pickup_GasBooster_C" _returnvalue "AlwaysSpawn" 0 0))
      (Development|PrintString (Utilities|GetDisplayName _returnvalue_2)))
    (:SPECIAL_1
      (bind _spawnlocation_2 (CallFunction|GetSpawnLocations (Variables|Default|GetspS1PickUpArray)))
      (bind _returnvalue_3 (CallFunction|PickUpOffSet _spawnlocation_2))
      (Game|SpawnActorfromClass "/Game/Blueprint/PickUp/BP_Pickup_GasBooster.BP_Pickup_GasBooster_C" _returnvalue_3 "AlwaysSpawn" 0 0))))

(fn PickUpOffSet
  (params (InTransform :type Transform%20%28by%20ref%29))
  (bind (_location _rotation _scale) (Math|Transform|BreakTransform InTransform))
  (bind (_x _y) (Math|Vector|BreakVector _location))
  (return (Math|Transform|MakeTransform (Math|Vector|MakeVector _x _y 1.5e+02) _rotation _scale)))