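; Save game controller that persists music and sound settings and the player's points in two separate slots.
; Each save function writes to its SaveGame object and slot; each load reads the slot or returns defaults if none exists.
; SavePointsData checks SaveSettings validity instead of SavePoints before creating its object.
; Points overwrite the previous save, as best-score comparison is still a TODO.
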(fn SaveSettingsData
  (params (isMusic :type Boolean) (isSound :type Boolean))
  (Utilities|IsValid (Variables|Default|GetSaveSettings)
    (:Is%20Valid
      _)
    (:Is%20Not%20Valid
      (bind _returnvalue (SaveGame|CreateSaveGameObject "/Game/Blueprint/SaveGame/SaveGame_Settings.SaveGame_Settings_C"))
      (Variables|Default|SetSaveSettings _returnvalue)))
  (Variables|/Game/Blueprint/SaveGame/SaveGame_Settings.SaveGame_Settings_C|SetisMusic (Variables|Default|GetSaveSettings) isMusic)
  (Variables|/Game/Blueprint/SaveGame/SaveGame_Settings.SaveGame_Settings_C|SetisSound (Variables|Default|GetSaveSettings) isSound)
  (SaveGame|SaveGametoSlot (Variables|Default|GetSaveSettings) (Variables|Default|GetSettingsDataSlotName)))

(fn LoadSettingsData
  (bind _returnvalue (SaveGame|DoesSaveGameExist (Variables|Default|GetSettingsDataSlotName)))
  (if _returnvalue
    (bind _returnvalue_2 (SaveGame|LoadGamefromSlot (Variables|Default|GetSettingsDataSlotName)))
    (bind _assave_game_settings (Utilities|Casting|CastToSaveGame_Settings _returnvalue_2))
    (return (Variables|/Game/Blueprint/SaveGame/SaveGame_Settings.SaveGame_Settings_C|GetisSound _assave_game_settings) (Variables|/Game/Blueprint/SaveGame/SaveGame_Settings.SaveGame_Settings_C|GetisMusic _assave_game_settings))
    (else
      (bind _returnvalue_3 (SaveGame|CreateSaveGameObject "/Game/Blueprint/SaveGame/SaveGame_Settings.SaveGame_Settings_C"))
      (Variables|Default|SetSaveSettings _returnvalue_3)
      (return true true))))

(fn SavePointsData
  (params (Points :type Float%20%28single-precision%29))
  ;[1 0.7953 0.3503] Must add a procedure to compare with the 3 best player games to determine if it is trully the best (Or just if its better than the last)
  (Utilities|IsValid (Variables|Default|GetSaveSettings)
    (:Is%20Valid
      _)
    (:Is%20Not%20Valid
      (bind _returnvalue (SaveGame|CreateSaveGameObject "/Game/Blueprint/SaveGame/SaveGame_Points.SaveGame_Points_C"))
      (bind _output_get (Variables|Default|SetSavePoints _returnvalue))))
  (Variables|/Game/Blueprint/SaveGame/SaveGame_Points.SaveGame_Points_C|SetPoints _output_get Points)
  (SaveGame|SaveGametoSlot _output_get (Variables|Default|GetPointsDataSlotName)))

(fn LoadPointsData
  (bind _returnvalue (SaveGame|DoesSaveGameExist (Variables|Default|GetPointsDataSlotName)))
  (if _returnvalue
    (bind _returnvalue_2 (SaveGame|LoadGamefromSlot (Variables|Default|GetPointsDataSlotName)))
    (bind _assave_game_points (Utilities|Casting|CastToSaveGame_Points _returnvalue_2))
    (return (Variables|/Game/Blueprint/SaveGame/SaveGame_Points.SaveGame_Points_C|GetPoints _assave_game_points))
    (else
      (bind _returnvalue_3 (SaveGame|CreateSaveGameObject "/Game/Blueprint/SaveGame/SaveGame_Points.SaveGame_Points_C"))
      (Variables|Default|SetSavePoints _returnvalue_3)
      (return 0.0))))