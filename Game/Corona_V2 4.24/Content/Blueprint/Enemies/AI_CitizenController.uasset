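; AI controller for citizen pawns that wander straight ahead until sent to a confinement point.
; Shortly after BeginPlay, a one-shot timer starts WalkForward, which repeatedly issues AIMoveTo just ahead of the pawn, retrying on success or failure.
; goToConfinedPoint clears that start timer, moves the pawn to the given destination and destroys it on arrival.
; Several disconnected movement nodes remain unused.
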(event Custom|goToConfinedPoint
  (params (Dest :type Vector%20%28by%20ref%29))
  (bind _returnvalue (Pawn|GetControlledPawn))
  (Utilities|Time|ClearandInvalidateTimerbyHandle (Variables|Default|GetwalkForwardTimer))
  (AI|AIMoveTo _returnvalue Dest 0 1e+02 false
    (:OnSuccess
      (Actor|DestroyActor _returnvalue))))

(event Custom|WalkForward
  (bind _returnvalue (Pawn|GetControlledPawn))
  (AI|AIMoveTo 0 (+ (Transformation|GetActorLocation _returnvalue) (* (Transformation|GetActorForwardVector _returnvalue) 1.5e+02)) 0 5e+01 false :!label _label
    (:OnSuccess
      (goto _label))
    (:OnFail
      (goto _label))))

(event EventBeginPlay
  (bind _returnvalue (Utilities|Time|SetTimerbyEvent (delegate Custom|WalkForward) 0.2))
  (Variables|Default|SetwalkForwardTimer _returnvalue))

(event EventTick
  (params (DeltaSeconds :type Float%20%28single-precision%29)))

(fn ConstructionScript)