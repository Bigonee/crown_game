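; Main menu player controller that shows the cursor, starts menu music and handles the menu widget's actions.
; BeginPlay creates a SaveGameController, loads settings and points, copies audio flags to GameInstanceCorona and sets the Music class volume through a sound mix override.
; It binds MainMenu widget events to open the mobile endless map, quit, or save changed audio settings.
; The PC level load is unwired and SyncWithLeaderboard is an empty stub.
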(event EventBeginPlay
  (bind _savegamecontroller (Variables|Default|GetSaveGameController))
  (Variables|Default|SetbShowMouseCursor true)
  (Utilities|FlowControl|Sequence
    (:then_0
      (CallFunction|CreateSaveLoadController))
    (:then_1
      (Class|GameplayStatics|SetBaseSoundMix "/Game/Sounds/GlobalSoundMix.GlobalSoundMix")
      (Audio|PlaySound2D "/Game/Sounds/src/background/bensound-funday_Cue.bensound-funday_Cue" 0.25 1.0 0.0 0 self))
    (:then_2
      (Utilities|FlowControl|Sequence
        (:then_0
          (bind (_issound _ismusic) (Default|LoadSettingsData _savegamecontroller))
          (bind _asgame_instance_corona (Utilities|Casting|CastToGameInstanceCorona (Game|GetGameInstance)))
          (Variables|/Game/Blueprint/GameInstanceCorona.GameInstanceCorona_C|SetisSound _asgame_instance_corona _issound)
          (bind _output_get (Variables|/Game/Blueprint/GameInstanceCorona.GameInstanceCorona_C|SetisMusic _asgame_instance_corona _ismusic))
          (if _output_get
            (Audio|SetSoundMixClassOverride "/Game/Sounds/GlobalSoundMix.GlobalSoundMix" "/Game/Sounds/Music.Music" 1.0 1.0 0.0 true)
            (else
              (Audio|SetSoundMixClassOverride "/Game/Sounds/GlobalSoundMix.GlobalSoundMix" "/Game/Sounds/Music.Music" 0.0 1.0 0.0 true))))
        (:then_1
          (Default|LoadPointsData _savegamecontroller))))
    (:then_3
      (|WidgetStuff))
    (:then_4
      (bind _asgame_instance_corona_2 (Utilities|Casting|CastToGameInstanceCorona (Game|GetGameInstance)))
      (Default|FakeBeginPlay _asgame_instance_corona_2))))

(event EventTick
  (params (DeltaSeconds :type Float%20%28single-precision%29)))

(fn ConstructionScript)

(fn CreateSaveLoadController
  (Utilities|IsValid (Variables|Default|GetSaveGameController)
    (:Is%20Not%20Valid
      (bind _returnvalue (Game|ConstructObjectfromClass "/Game/Blueprint/SaveGame/SaveGameController.SaveGameController_C" self))
      (Variables|Default|SetSaveGameController _returnvalue))))

(fn SyncwithLeaderboard)

(event Custom|OpenLevel_Event_0
  (Game|OpenLevel(byName) "EndlessMap_Mobile" false) ; Mobile Version
)

(event Custom|CloseGame_Event_0
  (Game|QuitGame (Game|GetPlayerController 0) "Quit" true))

(event Custom|UpdateAudioSettings_Event_0
  (params (isMusic :type Boolean) (isSound :type Boolean))
  (bind _asgame_instance_corona (Utilities|Casting|CastToGameInstanceCorona (Game|GetGameInstance)))
  (bind _output_get (Variables|/Game/Blueprint/GameInstanceCorona.GameInstanceCorona_C|SetisMusic _asgame_instance_corona isMusic))
  (bind _output_get_2 (Variables|/Game/Blueprint/GameInstanceCorona.GameInstanceCorona_C|SetisSound _asgame_instance_corona isSound))
  (Default|SaveSettingsData (Variables|Default|GetSaveGameController) _output_get _output_get_2))