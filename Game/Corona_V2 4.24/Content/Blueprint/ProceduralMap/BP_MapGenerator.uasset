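; Map generator that builds an endless road ahead of the player from chained tile actors, seeding a few at BeginPlay.
; The current tile number determines type (main road or one of four specials) and variant, selecting the Blueprint class to spawn.
; Each spawned tile supplies the next attach transform and binds an overlap dispatcher.
; When a PlayerPawn-tagged pawn triggers it, that tile is destroyed and a new one is appended.
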(event EventBeginPlay
  (for _index (range 0 2)
    (CallFunction|AddFloorTile)))

(event Collision|EventActorBeginOverlap
  (params (OtherActor :type Actor%20Object%20Reference)))

(event EventTick
  (params (DeltaSeconds :type Float%20%28single-precision%29)))

(fn ConstructionScript)

(fn AddFloorTile
  (bind _returnvalue (Class|MapGen|GetTileType (Variables|Default|GetcurrentTileNum)))
  (switch Utilities|FlowControl|Switch|SwitchonETileType _returnvalue
    (:MAIN
      (CallFunction|SpawnMain))
    (:SPECIAL_1
      (CallFunction|SpawnSpecial))
    (:SPECIAL_2
      (CallFunction|SpawnSpecial2))
    (:SPECIAL_3
      (CallFunction|SpawnSpecial3))
    (:SPECIAL_4
      (CallFunction|SpawnSpecial4))))

(fn GetAttachPointTransform
  (return ""))

(fn DestroyonOverlap
  (params (Pawn :type Actor%20Object%20Reference) (MapTile :type Actor%20Object%20Reference))
  (if (Actor|ActorHasTag Pawn "PlayerPawn")
    (Actor|DestroyActor MapTile)
    (CallFunction|AddFloorTile)))

(fn IncrementTileNum
  (Math|Integer|IncrementInt (Variables|Default|GetcurrentTileNum)))

(fn AfterSpawnTile
  (params (spawnedTile :type BP%20Tile%20Abstract%20Object%20Reference))
  (bind _attachtransform (Class|TileInterface|GetAttachPointTransform(Message) spawnedTile))
  (Variables|Default|SetNextSpawnPoint _attachtransform)
  (EventDispatchers|BindEventtoEvDispDestroyonOverlap spawnedTile (EventDispatchers|CreateEvent :!event DestroyonOverlap))
  (CallFunction|IncrementTileNum))

(fn SpawnMain
  (bind _returnvalue (Class|MapGen|GetTileVariant (Variables|Default|GetcurrentTileNum)))
  (switch int _returnvalue
    (:Default
      (bind _returnvalue_2 (Game|SpawnActorfromClass "/Game/Blueprint/ProceduralMap/Types/BP_road_2.BP_road_2_C" (Variables|Default|GetNextSpawnPoint) "Undefined" 0 (Variables|Default|GetcurrentTileNum) 1 0 :!label _label))
      (CallFunction|AfterSpawnTile _returnvalue_2))
    (:0
      (goto _label))
    (:1
      (bind _returnvalue_3 (Game|SpawnActorfromClass "/Game/Blueprint/ProceduralMap/Types/BP_road_3.BP_road_3_C" (Variables|Default|GetNextSpawnPoint) "Undefined" 0 (Variables|Default|GetcurrentTileNum) 1 0))
      (CallFunction|AfterSpawnTile _returnvalue_3))
    (:2
      (bind _returnvalue_4 (Game|SpawnActorfromClass "/Game/Blueprint/ProceduralMap/Types/BP_road_4.BP_road_4_C" (Variables|Default|GetNextSpawnPoint) "Undefined" 0 (Variables|Default|GetcurrentTileNum) 1 0))
      (CallFunction|AfterSpawnTile _returnvalue_4))
    (:3
      (bind _returnvalue_5 (Game|SpawnActorfromClass "/Game/Blueprint/ProceduralMap/Types/BP_road_1.BP_road_1_C" (Variables|Default|GetNextSpawnPoint) "Undefined" 0 (Variables|Default|GetcurrentTileNum) 1 0))
      (CallFunction|AfterSpawnTile _returnvalue_5))
    (:4
      (bind _returnvalue_6 (Game|SpawnActorfromClass "/Game/Blueprint/ProceduralMap/Types/BP_road_cross1.BP_road_cross1_C" (Variables|Default|GetNextSpawnPoint) "Undefined" 0 (Variables|Default|GetcurrentTileNum) 1 0))
      (CallFunction|AfterSpawnTile _returnvalue_6))))

(fn SpawnSpecial
  (bind _returnvalue (Class|MapGen|GetTileVariant (Variables|Default|GetcurrentTileNum)))
  (switch int _returnvalue
    (:Default
      (bind _returnvalue_2 (Game|SpawnActorfromClass "/Game/Blueprint/ProceduralMap/Types/BP_Special1_2.BP_Special1_2_C" (Variables|Default|GetNextSpawnPoint) "Undefined" 0 (Variables|Default|GetcurrentTileNum) 1 0 :!label _label))
      (CallFunction|AfterSpawnTile _returnvalue_2))
    (:0
      (bind _returnvalue_3 (Game|SpawnActorfromClass "/Game/Blueprint/ProceduralMap/Types/BP_Special1_1.BP_Special1_1_C" (Variables|Default|GetNextSpawnPoint) "Undefined" 0 (Variables|Default|GetcurrentTileNum) 1 0))
      (CallFunction|AfterSpawnTile _returnvalue_3))
    (:1
      (bind _returnvalue_4 (Game|SpawnActorfromClass "/Game/Blueprint/ProceduralMap/Types/BP_Special1_3.BP_Special1_3_C" (Variables|Default|GetNextSpawnPoint) "Undefined" 0 (Variables|Default|GetcurrentTileNum) 1 0))
      (CallFunction|AfterSpawnTile _returnvalue_4))
    (:2
      (goto _label))))

(fn SpawnSpecial2
  (bind _returnvalue (Class|MapGen|GetTileVariant (Variables|Default|GetcurrentTileNum)))
  (switch int _returnvalue
    (:Default
      (bind _returnvalue_2 (Game|SpawnActorfromClass "/Game/Blueprint/ProceduralMap/Types/BP_Special2_2.BP_Special2_2_C" (Variables|Default|GetNextSpawnPoint) "Undefined" 0 (Variables|Default|GetcurrentTileNum) 1 0 :!label _label))
      (CallFunction|AfterSpawnTile _returnvalue_2))
    (:0
      (bind _returnvalue_3 (Game|SpawnActorfromClass "/Game/Blueprint/ProceduralMap/Types/BP_Special2_1.BP_Special2_1_C" (Variables|Default|GetNextSpawnPoint) "Undefined" 0 (Variables|Default|GetcurrentTileNum) 1 0))
      (CallFunction|AfterSpawnTile _returnvalue_3))
    (:1
      (goto _label))))

(fn SpawnSpecial3
  (Class|MapGen|GetTileVariant (Variables|Default|GetcurrentTileNum))
  (bind _returnvalue (Game|SpawnActorfromClass "/Game/Blueprint/ProceduralMap/Types/BP_Special3_1.BP_Special3_1_C" (Variables|Default|GetNextSpawnPoint) "Undefined" 0 (Variables|Default|GetcurrentTileNum) 1 0))
  (CallFunction|AfterSpawnTile _returnvalue))

(fn SpawnSpecial4
  (Class|MapGen|GetTileVariant (Variables|Default|GetcurrentTileNum))
  (bind _returnvalue (Game|SpawnActorfromClass "/Game/Blueprint/ProceduralMap/Types/BP_Special4_1.BP_Special4_1_C" (Variables|Default|GetNextSpawnPoint) "Undefined" 0 (Variables|Default|GetcurrentTileNum) 1 0))
  (CallFunction|AfterSpawnTile _returnvalue))