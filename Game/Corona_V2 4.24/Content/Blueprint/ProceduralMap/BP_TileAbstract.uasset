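; Abstract base map tile for the procedural map, exposing an attach point transform and broadcasting a destroy-on-overlap event when its collision box is overlapped.
; The construction script scales car, group, citizen and trash counts by a difficulty multiplier.
; Empty spawn-point and confinement functions serve as stubs.
; Random-point enemy spawning by tile number remains but is disconnected, deprecated in favor of BP_EnemySpawner.
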(event OnComponentBeginOverlap(collisionBox)
  (params (OverlappedComponent :type Primitive%20Component%20Object%20Reference) (OtherActor :type Actor%20Object%20Reference) (OtherComp :type Primitive%20Component%20Object%20Reference) (OtherBodyIndex :type Integer) (bFromSweep :type Boolean) (SweepResult :type Hit%20Result%20Structure%20%28by%20ref%29))
  (Default|CallEvDispDestroyonOverlap OtherActor self))

(event EventBeginPlay)

(event Collision|EventActorBeginOverlap
  (params (OtherActor :type Actor%20Object%20Reference)))

(event EventTick
  (params (DeltaSeconds :type Float%20%28single-precision%29)))

(fn ConstructionScript
  (CallFunction|IncreaseSpawnIntensityDifficultyDriven))

(fn OnBeginOverlap)

(fn SetSpawnPoints
  (Utilities|FlowControl|Sequence
    (:then_0
      (SpawnPoints|SetSPCars))
    (:then_1
      (SpawnPoints|SetSPGroups))
    (:then_2
      (SpawnPoints|SetSPCharacters))
    (:then_3
      (SpawnPoints|SetSPTrash))))

(fn SetSPCars)

(fn SetSPGroups)

(fn SetSPCharacters)

(fn SpawnActors
  (if (not (== (Variables|Default|GettileNumber) 0))
    (Utilities|FlowControl|Sequence
      (:then_0
        (for _index (range 0 (Variables|EnemySpawn|GetNumOfCars))
          (bind _spawnlocation (SpawnEnemies|GetSpawnLocations (Variables|Default|GetspCarsArray)))
          (Game|SpawnActorfromClass "/Game/Blueprint/Enemies/Vehicles/EnemyPawn_vehicles.EnemyPawn_Vehicles_C" _spawnlocation "Undefined" 0 (Class|MapGen|GetVehicleType (Variables|Default|GettileNumber)) 0)))
      (:then_1
        (for _index_2 (range 0 (Variables|EnemySpawn|GetNumOfCitizen))
          (bind _spawnlocation_2 (SpawnEnemies|GetSpawnLocations (Variables|Default|GetspCharactersArray)))
          (Game|SpawnActorfromClass "/Game/Blueprint/Enemies/Citizens/EnemyPawn_Citizen.EnemyPawn_Citizen_C" _spawnlocation_2 "Undefined" 0 (Class|MapGen|GetCitzenType (Variables|Default|GettileNumber)) 0)))
      (:then_2
        (for _index_3 (range 0 (Variables|EnemySpawn|GetNumOfTrash))
          (bind _spawnlocation_3 (SpawnEnemies|GetSpawnLocations (Variables|Default|GetspTrashArray)))
          (Game|SpawnActorfromClass "/Game/Blueprint/Enemies/Trash/EnemyPawn_Trash.EnemyPawn_Trash_C" _spawnlocation_3 "Undefined" 0 (Class|MapGen|GetTrashType (Variables|Default|GettileNumber)) 0))))))

(fn GetSpawnLocations
  (params (SpawnPoints :type Array%20of%20Arrow%20Component%20Object%20References))
  (return (Transformation|GetWorldTransform (Utilities|Array|Get(acopy) SpawnPoints (Math|Random|RandomInteger (Utilities|Array|Length SpawnPoints))))))

(fn SpawnGroups
  (for _array_element (Variables|Default|GetspGroupsArray)
    (Game|SpawnActorfromClass "/Game/Blueprint/Enemies/Groups/EnemyPawn_Group.EnemyPawn_Group_C" (Transformation|GetWorldTransform _array_element) "Undefined" 0 (Class|MapGen|GetGroupType (Variables|Default|GettileNumber)) 0)))

(fn SpawnCharacters
  (for _array_element (Variables|Default|GetspCharactersArray)
    (Game|SpawnActorfromClass "/Game/Blueprint/Enemies/Citizens/EnemyPawn_Citizen.EnemyPawn_Citizen_C" (Transformation|GetWorldTransform _array_element) "Undefined" 0 (Class|MapGen|GetCitzenType (Variables|Default|GettileNumber)) 0)))

(fn SetSPTrash)

(fn SpawnTrash
  (for _array_element (Variables|Default|GetspTrashArray)
    (Game|SpawnActorfromClass "/Game/Blueprint/Enemies/Trash/EnemyPawn_Trash.EnemyPawn_Trash_C" (Transformation|GetWorldTransform _array_element) "Undefined" 0 (Class|MapGen|GetTrashType (Variables|Default|GettileNumber)) 0)))

(fn SetConfinedPoints)

(fn IncreaseSpawnIntensityDifficultyDriven
  (bind _dificultymultiplayer (Variables|EnemySpawn|GetDificultyMultiplayer))
  (Variables|EnemySpawn|SetNumOfCars (* (Variables|EnemySpawn|GetNumOfCars) _dificultymultiplayer))
  (Variables|EnemySpawn|SetNumOfGroups (* (Variables|EnemySpawn|GetNumOfGroups) _dificultymultiplayer))
  (Variables|EnemySpawn|SetNumOfCitizen (* (Variables|EnemySpawn|GetNumOfCitizen) _dificultymultiplayer))
  (Variables|EnemySpawn|SetNumOfTrash (* (Variables|EnemySpawn|GetNumOfTrash) _dificultymultiplayer)))

(fn EndBeginOverlap
  (params (OverlapActor :type Actor%20Object%20Reference))
  (return 0))

(fn GetAttachPointTransform
  (return (Transformation|GetWorldTransform (Variables|Default|GetattachPoint))))

(fn GetConfinedEvacuationPoint
  (params (enemyLocation :type Vector :default "0, 0, 0"))
  (return "0, 0, 0"))