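; Main menu player controller that shows the cursor, restores saved audio settings and opens the menu widget.
; On BeginPlay it creates a save-game controller, copies saved music and sound flags into the Corona game instance, and loads points data.
; Menu widget dispatchers open EndlessMap, quit the game, or push audio changes to the game instance and save them.
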(event EventBeginPlay
  (bind _savegamecontroller (Variables|Default|GetSaveGameController))
  (Variables|Default|SetbShowMouseCursor true)
  (Utilities|FlowControl|Sequence
    (:then_0
      (CallFunction|CreateSaveLoadController))
    (:then_1
      (Utilities|FlowControl|Sequence
        (:then_0
          (bind (_issound _ismusic) (Default|LoadSettingsData _savegamecontroller))
          (bind _asgame_instance_corona (Utilities|Casting|CastToGameInstanceCorona (Game|GetGameInstance)))
          (Variables|/Game/Blueprint/GameInstanceCorona.GameInstanceCorona_C|SetisSound _asgame_instance_corona _issound)
          (Variables|/Game/Blueprint/GameInstanceCorona.GameInstanceCorona_C|SetisMusic _asgame_instance_corona _ismusic))
        (:then_1
          (Default|LoadPointsData _savegamecontroller))))
    (:then_2
      (|WidgetStuff))))

(event EventTick
  (params (DeltaSeconds :type Float%20%28single-precision%29)))

(fn ConstructionScript)

(fn CreateSaveLoadController
  (Utilities|IsValid (Variables|Default|GetSaveGameController)
    (:Is%20Not%20Valid
      (bind _returnvalue (Game|ConstructObjectfromClass "/Game/Blueprint/SaveGame/SaveGameController.SaveGameController_C" self))
      (Variables|Default|SetSaveGameController _returnvalue))))

(event Custom|OpenLevel_Event_0
  (Game|OpenLevel(byName) "EndlessMap"))

(event Custom|CloseGame_Event_0
  (Game|QuitGame 0 "Quit" false))

(event Custom|UpdateAudioSettings_Event_0
  (params (isMusic :type Boolean) (isSound :type Boolean))
  (bind _asgame_instance_corona (Utilities|Casting|CastToGameInstanceCorona (Game|GetGameInstance)))
  (bind _output_get (Variables|/Game/Blueprint/GameInstanceCorona.GameInstanceCorona_C|SetisMusic _asgame_instance_corona isMusic))
  (bind _output_get_2 (Variables|/Game/Blueprint/GameInstanceCorona.GameInstanceCorona_C|SetisSound _asgame_instance_corona isSound))
  (Default|SaveSettingsData (Variables|Default|GetSaveGameController) _output_get _output_get_2))