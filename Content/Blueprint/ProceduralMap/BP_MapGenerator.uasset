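; BP_MapGenerator builds an endless street by spawning a starting run of BP_Tile_Street actors at BeginPlay.
; Each tile spawns at the previous tile's attach point with the current theme, which alternates between two values by tile-count parity.
; The generator binds to each tile's overlap event, with DestroyOnOverlap destroying tiles touched by the tagged player pawn and appending a new one.
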(event EventBeginPlay
  (for _index (range 0 9)
    (CallFunction|AddFloorTile)))

(event Collision|EventActorBeginOverlap
  (params (OtherActor :type Actor%20Object%20Reference)))

(event EventTick
  (params (DeltaSeconds :type Float%20%28single-precision%29)))

(fn ConstructionScript)

(fn AddFloorTile
  (bind _returnvalue (Game|SpawnActorfromClass "/Game/Blueprint/ProceduralMap/BP_Tile_Street.BP_Tile_Street_C" (Variables|Default|GetNextSpawnPoint) "Undefined" 0 (Variables|Default|GetcurrentTileTheme) 0))
  (Utilities|FlowControl|Sequence
    (:then_0
      (bind _attachtransform (Class|TileInterface|GetAttachPointTransform(Message) _returnvalue))
      (Variables|Default|SetNextSpawnPoint _attachtransform)
      (EventDispatchers|BindEventtoEvDispDestroyonOverlap _returnvalue (EventDispatchers|CreateEvent :!event DestroyonOverlap)))
    (:then_1
      (CallFunction|IncrementTileNum)
      (CallFunction|SetTheme))))

(fn GetAttachPointTransform
  (return "" ""))

(fn DestroyonOverlap
  (params (Pawn :type Actor%20Object%20Reference) (MapTile :type Actor%20Object%20Reference))
  (if (Actor|ActorHasTag Pawn "PlayerPawn")
    (Actor|DestroyActor MapTile)
    (CallFunction|AddFloorTile)))

(fn IncrementTileNum
  (Math|Integer|IncrementInt (Variables|Default|GettileNum)))

(fn SetTheme
  (if (== (.Remainder (Math|Float|Division(WholeandRemainder) (Math|Conversions|ToFloat(Integer) (Variables|Default|GettileNum)) 2.0)) 0.0)
    (Variables|Default|SetcurrentTileTheme "NewEnumerator0")
    (else
      (Variables|Default|SetcurrentTileTheme "NewEnumerator1"))))