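; BP_MapTile is a map tile piece for procedural map building, exposing its AttachPoint world transform through GetAttachTrans.
; When an actor overlaps EndTrigger and its IsOverlapingMessage check returns true, it fires the EvDispDestroyOnOverlap dispatcher with that actor and itself.
; The construction script switches on Tematica, but its FloorMesh mesh-setting nodes are disconnected.
; EndBeginOverlap is an empty stub.
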(event OnComponentBeginOverlap(EndTrigger)
  (params (OverlappedComponent :type Primitive%20Component%20Object%20Reference) (OtherActor :type Actor%20Object%20Reference) (OtherComp :type Primitive%20Component%20Object%20Reference) (OtherBodyIndex :type Integer) (bFromSweep :type Boolean) (SweepResult :type Hit%20Result%20Structure%20%28by%20ref%29))
  (bind _isoverlaping_ (Class|PawnInterface|IsOverlaping?(Message) OtherActor))
  (if _isoverlaping_
    (Default|CallEvDispDestroyonOverlap OtherActor self)))

(event EventBeginPlay)

(event Collision|EventActorBeginOverlap
  (params (OtherActor :type Actor%20Object%20Reference)))

(event EventTick
  (params (DeltaSeconds :type Float%20%28single-precision%29)))

(fn ConstructionScript
  (switch Utilities|FlowControl|Switch|SwitchonEN_Tematica (Variables|Default|GetTematica)))

(fn EndBeginOverlap
  (params (OverlapActor :type Actor%20Object%20Reference))
  (return 0))

(fn GetAttachTrans
  (return (Transformation|GetWorldTransform (Variables|Default|GetAttachPoint))))