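; Player controller for the main menu that shows the mouse cursor, restores saved audio settings and opens the menu.
; On BeginPlay it creates a SaveGameController object if needed, then copies the saved sound and music flags into GameInstanceCorona.
; It then adds the MainMenu widget to the viewport and binds its dispatchers to open EndlessMap or quit the game.
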(event Custom|OpenLevel_Event_0
  (Game|OpenLevel(byName) "EndlessMap"))

(event Custom|CloseGame_Event_0
  (Game|QuitGame 0 "Quit" false))

(event EventBeginPlay
  (Variables|Default|SetbShowMouseCursor true)
  (Utilities|FlowControl|Sequence
    (:then_0
      (CallFunction|CreateSaveLoadController))
    (:then_1
      (bind (_issound _ismusic) (Default|LoadSettingsData (Variables|Default|GetSaveGameController)))
      (bind _asgame_instance_corona (Utilities|Casting|CastToGameInstanceCorona (Game|GetGameInstance)))
      (Variables|/Game/Blueprint/GameInstanceCorona.GameInstanceCorona_C|SetisSound _asgame_instance_corona _issound)
      (Variables|/Game/Blueprint/GameInstanceCorona.GameInstanceCorona_C|SetisMusic _asgame_instance_corona _ismusic))
    (:then_2
      (bind _returnvalue (UserInterface|CreateWidget "/Game/Widget/MainMenu.MainMenu_C"))
      (UserInterface|Viewport|AddtoViewport _returnvalue 0)
      (EventDispatchers|AssignOpenLevel _returnvalue (delegate Custom|OpenLevel_Event_0))
      (EventDispatchers|AssignCloseGame _returnvalue (delegate Custom|CloseGame_Event_0)))))

(event EventTick
  (params (DeltaSeconds :type Float%20%28single-precision%29)))

(fn ConstructionScript)

(fn CreateSaveLoadController
  (Utilities|IsValid (Variables|Default|GetSaveGameController)
    (:Is%20Not%20Valid
      (bind _returnvalue (Game|ConstructObjectfromClass "/Game/Blueprint/SaveGame/SaveGameController.SaveGameController_C" self))
      (Variables|Default|SetSaveGameController _returnvalue))))