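; Save-game controller that persists the player's sound effects and audio on/off settings.
; Saving writes both flags into a settings save object, creating one if needed, and stores it in a named slot.
; Loading reads the flags from that slot, or creates a fresh save object and returns both as enabled when no save exists.
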(fn SaveSettingsData
  (params (isSoundEffect :type Boolean) (isAudio :type Boolean))
  (Utilities|IsValid (Variables|Default|GetSaveSettings)
    (:Is%20Valid
      _)
    (:Is%20Not%20Valid
      (bind _returnvalue (SaveGame|CreateSaveGameObject "/Game/Blueprint/SaveGame/SaveGame_Settings.SaveGame_Settings_C"))
      (Variables|Default|SetSaveSettings _returnvalue)))
  (Variables|/Game/Blueprint/SaveGame/SaveGame_Settings.SaveGame_Settings_C|SetisSoundEffects (Variables|Default|GetSaveSettings) isSoundEffect)
  (Variables|/Game/Blueprint/SaveGame/SaveGame_Settings.SaveGame_Settings_C|SetisAudio (Variables|Default|GetSaveSettings) isAudio)
  (SaveGame|SaveGametoSlot (Variables|Default|GetSaveSettings) (Variables|Default|GetSettingsDataSlotName)))

(fn LoadSettingsData
  (bind _returnvalue (SaveGame|DoesSaveGameExist (Variables|Default|GetSettingsDataSlotName)))
  (if _returnvalue
    (bind _returnvalue_2 (SaveGame|LoadGamefromSlot (Variables|Default|GetSettingsDataSlotName)))
    (bind _assave_game_settings (Utilities|Casting|CastToSaveGame_Settings _returnvalue_2))
    (return (Variables|/Game/Blueprint/SaveGame/SaveGame_Settings.SaveGame_Settings_C|GetisSoundEffects _assave_game_settings) (Variables|/Game/Blueprint/SaveGame/SaveGame_Settings.SaveGame_Settings_C|GetisAudio _assave_game_settings))
    (else
      (bind _returnvalue_3 (SaveGame|CreateSaveGameObject "/Game/Blueprint/SaveGame/SaveGame_Settings.SaveGame_Settings_C"))
      (Variables|Default|SetSaveSettings _returnvalue_3)
      (return true true))))