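; Enemy car pawn that takes its visible body from a selectable car type.
; The construction script switches on the ENCarType enum and assigns a sports car, pickup or box truck mesh to its static mesh component, so the choice shows in the editor.
; The event graph holds only disabled default events, so this Blueprint adds no runtime logic of its own.
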(event EventBeginPlay
  (|CallParentFunction) ; This node is disabled and will not be called.\nDrag off pins to build functionality.
)

(event Collision|EventActorBeginOverlap
  (params (OtherActor :type Actor%20Object%20Reference))
  (|CallParentFunction OtherActor) ; This node is disabled and will not be called.\nDrag off pins to build functionality.
)

(event EventTick
  (params (DeltaSeconds :type Float%20%28single-precision%29))
  (|CallParentFunction DeltaSeconds) ; This node is disabled and will not be called.\nDrag off pins to build functionality.
)

(fn ConstructionScript
  (bind _staticmesh (Variables|Default|GetStaticMesh))
  (|CallParentFunction)
  (switch Utilities|FlowControl|Switch|SwitchonEN_CarTypes (Variables|Default|GetEN_CarType)
    (:NewEnumerator0
      (Components|StaticMesh|SetStaticMesh _staticmesh "/Game/VehicleVarietyPack/Meshes/SM_SportsCar.SM_SportsCar"))
    (:NewEnumerator1
      (Components|StaticMesh|SetStaticMesh _staticmesh "/Game/VehicleVarietyPack/Meshes/SM_Pickup.SM_Pickup"))
    (:NewEnumerator2
      (Components|StaticMesh|SetStaticMesh _staticmesh "/Game/VehicleVarietyPack/Meshes/SM_Truck_Box.SM_Truck_Box"))))