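; Player controller for gameplay that creates the in-game UI and relays its move and jump buttons to the pawn through messages.
; HP and infection updates refresh the progress bars and, when HP empties or infection maxes out, trigger pawn death and the end-game UI.
; Touch taps message the actor under the cursor as an enemy tap.
; Replay reloads EndlessMap; perk buttons only print, and menu and publish button handlers are empty.
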(event Custom|Replay
  ;[1 1 1] POPUP UI Buttons
  (Game|OpenLevel(byName) "EndlessMap"))

(event Custom|GoToMenu
  ;[1 1 1] POPUP UI Buttons
  (Game|OpenLevel(byName) "MainMap"))

(event Custom|Publish
  ;[1 1 1] POPUP UI Buttons
)

(event EventBeginPlay
  ;[1 1 1] Begin Play Logic
  (Variables|Default|SetbShowMouseCursor true)
  (Utilities|FlowControl|Sequence
    (:then_1
      (|WIDGETStuff))
    (:then_2
      (Default|UpdateProgressBars (Variables|Default|GetInGameUI) 100) ; Setup Begin Play Variables
    )))

(event EventUpdateHpInfection
  (params (HP :type Integer) (Infection :type Integer))
  ;[1 1 1] HP - Infection Data Flow
  (Default|UpdateProgressBars (Variables|Default|GetInGameUI) HP Infection)
  (bind _returnvalue (CallFunction|CheckifEndGame HP Infection))
  (if _returnvalue
    (Class|PawnInterface|OnDieEndGame(Message) (Game|Player|GetPlayerPawn 0))
    (Default|SetupEndGame (Variables|Default|GetInGameUI))))

(event Input|KeyboardEvents|X
  (params (Key :type Key%20Structure))
  (:Pressed
    (Default|UpdateProgressBars (Variables|Default|GetInGameUI) 25 75)))

(event Input|TouchEvents|Touch1
  (params (Key :type Key%20Structure))
  ;[1 0.2292 0.2292] DEPRECATED - Move Input Touch Screen + OribtCam
)

(event Input|TouchEvents|Touch1
  (params (Key :type Key%20Structure))
  (:Pressed
    (Class|EnemyInterface|CallEnemyTap(Message) (.HitActor (Collision|BreakHitResult (.HitResult (Game|Player|GetHitResultUnderCursorbyChannel "TraceTypeQuery1" true)))))))

(fn ConstructionScript)

(fn CheckifEndGame
  (params (HP :type Integer) (InfectionAmount :type Integer))
  (return (or (<= HP 0) (>= InfectionAmount (Variables|Default|GetMaxInfectionValue)))))

(event Custom|MoveRight_Event_0
  (params (isPressed :type Boolean))
  ;[1 1 1] Move Actions
  (Class|PawnInterface|CallMoveRight(Message) (Game|Player|GetPlayerPawn 0) isPressed))

(event Custom|MoveLeft_Event_0
  (params (isPressed :type Boolean))
  ;[1 1 1] Move Actions
  (Class|PawnInterface|CallMoveLeft(Message) (Game|Player|GetPlayerPawn 0) isPressed))

(event Custom|Jump_Event_0
  (params (isPressed :type Boolean))
  ;[1 1 1] Move Actions
  (Class|PawnInterface|CallJump(Message) (Game|Player|GetPlayerPawn 0) isPressed))

(event Custom|GoToMenu_Event_0
  ;[1 1 1] On Die PopUp UI
)

(event Custom|Replay_Event_0
  ;[1 1 1] On Die PopUp UI
  (CallFunction|Replay))

(event Custom|Publish_Event_0
  ;[1 1 1] On Die PopUp UI
)

(event Custom|PerkLeft_Event_0
  ;[1 1 1] Perks Actions
  (Development|PrintString "Action Perk LEFT"))

(event Custom|PerkRight_Event_0
  ;[1 1 1] Perks Actions
  (Development|PrintString "Action Perk RIGHT"))